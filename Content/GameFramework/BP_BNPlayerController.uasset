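; Player controller Blueprint that binds keys for opening the inventory and for adding and using move-speed tarot card items, apparently as test input.
; Key 2 adds and key 3 uses one card through the player state's InventoryComponent, looked up by gameplay tag.
; Each key has its own FlipFlop alternating between the Up and Down cards.
; Tab alternates between creating the inventory widget and removing it from its parent.
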(event Input|KeyboardEvents|2
  (params (Key :type Key%20Structure :default "None"))
  (:Pressed
    (bind _asbp_bnplayer_state (Utilities|Casting|CastToBP_BNPlayerState (Variables|/Script/Engine.Controller|GetPlayerState (Game|GetPlayerController 0))))
    (Utilities|FlowControl|FlipFlop
      (:A
        (Class|InventoryComponent|AddItembyTag (Variables|/Script/BigNightmares.BNPlayerState|GetInventoryComponent _asbp_bnplayer_state) (GameplayTags|MakeLiteralGameplayTag "(TagName=\"Item.TarotCard.MoveSpeed.Up\")") 1))
      (:B
        (Class|InventoryComponent|AddItembyTag (Variables|/Script/BigNightmares.BNPlayerState|GetInventoryComponent _asbp_bnplayer_state) (GameplayTags|MakeLiteralGameplayTag "(TagName=\"Item.TarotCard.MoveSpeed.Down\")") 1)))))

(event Input|KeyboardEvents|3
  (params (Key :type Key%20Structure :default "None"))
  (:Pressed
    (bind _asbp_bnplayer_state (Utilities|Casting|CastToBP_BNPlayerState (Variables|/Script/Engine.Controller|GetPlayerState (Game|GetPlayerController 0))))
    (Utilities|FlowControl|FlipFlop
      (:A
        (Class|InventoryComponent|UseItembyTag (Variables|/Script/BigNightmares.BNPlayerState|GetInventoryComponent _asbp_bnplayer_state) (GameplayTags|MakeLiteralGameplayTag "(TagName=\"Item.TarotCard.MoveSpeed.Up\")") 1))
      (:B
        (Class|InventoryComponent|UseItembyTag (Variables|/Script/BigNightmares.BNPlayerState|GetInventoryComponent _asbp_bnplayer_state) (GameplayTags|MakeLiteralGameplayTag "(TagName=\"Item.TarotCard.MoveSpeed.Down\")") 1)))))

(event Input|KeyboardEvents|Tab
  (params (Key :type Key%20Structure :default "None"))
  (bind _inventorywidget (Variables|Default|GetInventoryWidget))
  (:Pressed
    (Utilities|FlowControl|FlipFlop
      (:A
        (Class|BNPlayerController|CreateInventoryWidget))
      (:B
        (Utilities|IsValid _inventorywidget
          (:Is%20Valid
            (Widget|RemovefromParent _inventorywidget)))))))

(fn ConstructionScript)