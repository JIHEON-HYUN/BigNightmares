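; Player controller that shows win screens and mission widgets and relays mission player lists in a game with Prey and Resident sides.
; On the local controller, game end shows the winning side's screen for five seconds, and a mission event opens a transition widget with its player list, closed by a separate event.
; Ready-state changes find the tagged mission portal matching the mission type and pass it the new player list.
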(event Custom|CreateGameEndWidget
  (params (IsPreyWin :type Boolean))
  (if IsPreyWin
    (if (Pawn|IsLocalPlayerController)
      (bind _returnvalue (UserInterface|CreateWidget "/Game/UI/InGame/ResultUI/WBP_PreyWin.WBP_PreyWin_C" self))
      (UserInterface|Viewport|AddtoViewport _returnvalue 0)
      (Utilities|FlowControl|Delay 5.0)
      (Widget|RemovefromParent _returnvalue))
    (elif (Pawn|IsLocalPlayerController)
      (bind _returnvalue_2 (UserInterface|CreateWidget "/Game/UI/InGame/ResultUI/WBP_ResidentWin.WBP_ResidentWin_C" self))
      (UserInterface|Viewport|AddtoViewport _returnvalue_2 0)
      (Utilities|FlowControl|Delay 5.0)
      (Widget|RemovefromParent _returnvalue_2))))

(event Custom|CreateMissionWidget
  (params (MissionType :type E_MissionType%20Enum :default "NewEnumerator0") (MissionPlayerList :type Array%20of%20ST%20Mission%20Player%20Structures))
  (bind _self self)
  (if (Pawn|IsLocalPlayerController _self)
    (bind _returnvalue (UserInterface|CreateWidget "/Game/UI/InGame/Mission/MissionTransition/WBP_MissionTransition.WBP_MissionTransition_C" _self MissionType))
    (bind _output_get (Variables|Default|SetMissionWidget _returnvalue))
    (Default|SetPlayerList _output_get MissionPlayerList)
    (Default|OpenMenu _output_get)))

(event Custom|ChangeReadyState
  (params (MissionType :type E_MissionType%20Enum :default "NewEnumerator0") (NewPlayerList :type Array%20of%20ST%20Mission%20Player%20Structures))
  (switch Utilities|FlowControl|Switch|SwitchonE_MissionType MissionType
    (:NewEnumerator0
      (bind _outactors (Actor|GetAllActorsOfClasswithTag "/Game/MissionActor/MissionPortal/BP_MissionPortal.BP_MissionPortal_C" "PrivateMission"))
      (Default|SetMissionPlayerList (Utilities|Array|Get(acopy) _outactors) NewPlayerList))
    (:NewEnumerator1
      (bind _outactors_2 (Actor|GetAllActorsOfClasswithTag "/Game/MissionActor/MissionPortal/BP_MissionPortal.BP_MissionPortal_C" "CooperativeMission"))
      (Default|SetMissionPlayerList (Utilities|Array|Get(acopy) _outactors_2) NewPlayerList))
    (:NewEnumerator2
      (bind _outactors_3 (Actor|GetAllActorsOfClasswithTag "/Game/MissionActor/MissionPortal/BP_MissionPortal.BP_MissionPortal_C" "SacrificeMission"))
      (Default|SetMissionPlayerList (Utilities|Array|Get(acopy) _outactors_3) NewPlayerList))
    (:NewEnumerator3
      (bind _outactors_4 (Actor|GetAllActorsOfClasswithTag "/Game/MissionActor/MissionPortal/BP_MissionPortal.BP_MissionPortal_C" "AssignableMission"))
      (Default|SetMissionPlayerList (Utilities|Array|Get(acopy) _outactors_4) NewPlayerList))))

(event Custom|CloseMissionWidget
  (Default|CloseMenu (Variables|Default|GetMissionWidget)))

(fn ConstructionScript)