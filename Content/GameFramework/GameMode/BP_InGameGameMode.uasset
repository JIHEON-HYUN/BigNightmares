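; BP_InGameGameMode is the in-game game mode that runs missions, currently the Sacrifice Mission.
; LoadMissionLevel stores the player states, starts streaming L_SacrificeMission without blocking, and immediately moves two pawns to fixed mission positions.
; SacrificeMissionEnd marks the named player alive through BP_GameState, requests the unload and moves both pawns to one shared point near the origin.
; The unload names the level "SacrificeMission", without the L_ prefix used on load.
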(event Custom|LoadMissionLevel
  (params (MissionType :type E_MissionType%20Enum :default "NewEnumerator0") (MissionPlayerState :type Array%20of%20BP%20Player%20State%20Object%20References))
  (Variables|Default|SetMission%20Player%20State MissionPlayerState)
  (switch Utilities|FlowControl|Switch|SwitchonE_MissionType MissionType
    (:NewEnumerator2
      (Game|LoadStreamLevel(byName) "L_SacrificeMission" true)
      (Transformation|SetActorLocation (PlayerState|GetPawn (Utilities|Array|Get(acopy) (Variables|Default|GetMission%20Player%20State))) "50.000000,10267.000000,983.000000" false false)
      (Transformation|SetActorLocation (PlayerState|GetPawn (Utilities|Array|Get(acopy) (Variables|Default|GetMission%20Player%20State) 1)) "50.000000,9713.000000,983.000000" false false))))

(event Custom|UnLoadMissionLevel
  (params (MissionType :type E_MissionType%20Enum :default "NewEnumerator0"))
  (switch Utilities|FlowControl|Switch|SwitchonE_MissionType MissionType
    (:NewEnumerator2
      (Game|UnloadStreamLevel(byName) "SacrificeMission" false))))

(fn ConstructionScript)

(fn SacrificeMissionEnd
  (params (PlayerName :type String))
  (bind _asbp_game_state (Utilities|Casting|CastToBP_GameState (Game|GetGameState)))
  (Class|BNGameState|SetPlayerStatusAlive _asbp_game_state PlayerName)
  (CallFunction|UnLoadMissionLevel "NewEnumerator2")
  (Transformation|SetActorLocation (PlayerState|GetPawn (Utilities|Array|Get(acopy) (Variables|Default|GetMission%20Player%20State))) "0.000000,0.000000,100.000000" false false)
  (Transformation|SetActorLocation (PlayerState|GetPawn (Utilities|Array|Get(acopy) (Variables|Default|GetMission%20Player%20State) 1)) "0.000000,0.000000,100.000000" false false))