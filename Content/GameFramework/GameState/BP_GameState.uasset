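; In-match game state that propagates player deaths and handles the end of a game with a prey win or loss.
; On BeginPlay it binds to the in-game player list update, then matches entries to BP_PlayerState actors by name and calls PlayerDead on dead players' BP_TestMono pawns.
; GameEnd creates the result widget on each BP_PlayerController and calls the game mode's ReturnToLobby inside that same per-player loop.
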(event Custom|SetPlayerDead
  (params (NewList :type Array%20of%20In%20Game%20Player%20Data%20Structures))
  (for _array_element (Variables|Default|GetInGamePlayerDataList)
    (bind _outactors (Actor|GetAllActorsOfClass "/Game/GameFramework/PlayerState/BP_PlayerState.BP_PlayerState_C"))
    (for _array_element_2 _outactors
      (if (Utilities|Enum|Equal(Enum) (.playername _array_element) (PlayerState|GetPlayerName _array_element_2))
        (if (not (.bstatusalive _array_element))
          (bind _asbp_test_mono (Utilities|Casting|CastToBP_TestMono (PlayerState|GetPawn _array_element_2)))
          (Default|PlayerDead _asbp_test_mono))))))

(event EventBeginPlay
  (EventDispatchers|BindEventtoOninGamePlayerUpdated (delegate Custom|SetPlayerDead)))

(event EventGameEnd
  (params (bIsPreyWin :type Boolean))
  (for _array_element (Variables|Default|GetPlayerArray)
    (bind _asbp_player_controller (Utilities|Casting|CastToBP_PlayerController (Game|GetPlayerController _array_element)))
    (Default|CreateGameEndWidget _asbp_player_controller bIsPreyWin)
    (bind _asbp_in_game_game_mode (Utilities|Casting|CastToBP_InGameGameMode (Game|GetGameMode)))
    (Class|BNinGameGameMode|ReturntoLobby _asbp_in_game_game_mode)))

(fn ConstructionScript)