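; Test player character with a follow camera that fades static-mesh actors blocking its view of the character.
; Tick runs a delayed camera-to-mesh trace, accumulates hit actors and sets "Hide" to 0.3 on new dynamic material instances, with no restore step.
; Camera events reparent the camera to the boom or a "MissionCamera"-tagged actor's camera.
; On BeginPlay, the locally controlled pawn broadcasts initial values after a delay, longer on remote clients.
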(event Custom|InGameCameraInit
  (Transformation|AttachComponentToComponent (Variables|Default|GetFollowCamera) (Variables|Default|GetCameraBoom) "None" "KeepRelative" "KeepRelative" "KeepRelative" true))

(event Custom|ClientInitDelayFinished
  (Class|BNMonoCharacter|BroadcastInitialValues))

(event Custom|ClientInitDelay
  (Utilities|Time|SetTimerbyEvent (delegate Custom|ClientInitDelayFinished) 1.0))

(event Custom|MissionCameraInit
  (bind _outactors (Actor|GetAllActorswithTag "MissionCamera"))
  (Utilities|IsValid (Utilities|Array|Get(acopy) _outactors)
    (:Is%20Valid
      (Transformation|AttachComponentToComponent (Variables|Default|GetFollowCamera) (Actor|GetComponentbyClass (Utilities|Array|Get(acopy) _outactors) "/Script/Engine.CameraComponent") "None" "KeepRelative" "KeepRelative" "KeepRelative" true))))

(event EventTick
  (params (DeltaSeconds :type Float%20%28single-precision%29))
  (Utilities|FlowControl|Delay 0.1)
  (Utilities|Array|Clear (Variables|Default|GetHitActorsThisTick))
  (bind (_outhit _returnvalue) (Collision|LineTraceByChannel (Transformation|GetWorldLocation (Variables|Default|GetFollowCamera)) (Transformation|GetWorldLocation (Variables|Character|GetMesh)) "TraceTypeQuery3" false (Utilities|Array|MakeArray self) "ForDuration"))
  (Utilities|IsValid (.HitActor (Collision|BreakHitResult _outhit))
    (:Is%20Valid
      (if _returnvalue
        (Utilities|Array|AddUnique (Variables|Default|GetHitActorsThisTick) (.HitActor (Collision|BreakHitResult _outhit)))
        (for _array_element (Variables|Default|GetHitActorsThisTick)
          (if (not (Utilities|Array|ContainsItem (Variables|Default|GetCurrentlyHitObject) _array_element))
            (Utilities|Array|AddUnique (Variables|Default|GetCurrentlyHitObject) _array_element)))
        (for _array_element_2 (Variables|Default|GetCurrentlyHitObject)
          (CallFunction|SetActorOpacity _array_element_2 0.3))))))

(event EventBeginPlay
  (if (Pawn|IsLocallyControlled)
    (Utilities|FlowControl|Delay 0.2)
    (Networking|SwitchHasAuthority
      (:Authority
        (Class|BNMonoCharacter|BroadcastInitialValues))
      (:Remote
        (CallFunction|ClientInitDelay)))))

(fn ConstructionScript)

(fn SetActorOpacity
  (params (TargetActor :type Actor%20Object%20Reference) (NewOpacity :type Float%20%28double-precision%29))
  (for (_array_element _array_index) (Actor|GetComponentsByClass TargetActor "/Script/Engine.StaticMeshComponent")
    (bind _returnvalue (Rendering|Material|CreateDynamicMaterialInstance _array_element 0 (Rendering|Material|GetMaterial _array_element _array_index) "None" :!class /Script/Engine.PrimitiveComponent))
    (Rendering|Material|SetScalarParameterValue _returnvalue "Hide" NewOpacity :!class /Script/Engine.MaterialInstanceDynamic)))