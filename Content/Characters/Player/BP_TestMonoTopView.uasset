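; Test top-view player character with a follow camera that can switch between in-game and mission views.
; When locally controlled, it broadcasts initial values after a short delay, with an extra timer wait on clients.
; Camera events reattach FollowCamera to the boom or to the camera on the first MissionCamera-tagged actor.
; A line-trace routine for fading actors between camera and mesh is present but disconnected.
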(event Custom|InGameCameraInit
  (Transformation|AttachComponentToComponent (Variables|Default|GetFollowCamera) (Variables|Default|GetCameraBoom) "None" "KeepRelative" "KeepRelative" "KeepRelative" true))

(event Custom|ClientInitDelayFinished
  (Class|BNMonoCharacter|BroadcastInitialValues))

(event Custom|ClientInitDelay
  (Utilities|Time|SetTimerbyEvent (delegate Custom|ClientInitDelayFinished) 1.0))

(event Custom|MissionCameraInit
  (bind _outactors (Actor|GetAllActorswithTag "MissionCamera"))
  (Utilities|IsValid (Utilities|Array|Get(acopy) _outactors)
    (:Is%20Valid
      (Transformation|AttachComponentToComponent (Variables|Default|GetFollowCamera) (Actor|GetComponentbyClass (Utilities|Array|Get(acopy) _outactors) "/Script/Engine.CameraComponent") "None" "KeepRelative" "KeepRelative" "KeepRelative" true))))

(event Custom|CustomEvent
  (params (DeltaSeconds :type Float%20%28single-precision%29)))

(event EventBeginPlay
  (if (Pawn|IsLocallyControlled)
    (Utilities|FlowControl|Delay 0.2)
    (Networking|SwitchHasAuthority
      (:Authority
        (Class|BNMonoCharacter|BroadcastInitialValues))
      (:Remote
        (CallFunction|ClientInitDelay)))))

(fn ConstructionScript)