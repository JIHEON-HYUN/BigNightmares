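; BP_TestMono is a player character Blueprint, apparently for testing, that broadcasts initial values and shows a debug readout of movement speed.
; After BeginPlay, the locally controlled instance waits briefly, then calls BroadcastInitialValues immediately on authority or after a further timer delay on remote clients.
; Tick writes the CharacterMovement MaxWalkSpeed into its WBP_DebugSpeed widget to verify that speed changes apply.
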(event Custom|ClientInitDelay
  (Utilities|Time|SetTimerbyEvent (delegate Custom|ClientInitDelayFinished) 1.0))

(event Custom|ClientInitDelayFinished
  (Class|BNMonoCharacter|BroadcastInitialValues))

(event EventTick
  (params (DeltaSeconds :type Float%20%28single-precision%29))
  ;[1 1 1] tick을 활용해 디버깅중 속도 잘 바뀌면 문제없음
  (bind _aswbp_debug_speed (Utilities|Casting|CastToWBP_DebugSpeed (UserInterface|GetUserWidgetObject (Variables|Default|GetWidget))))
  (Rendering|Components|TextRender|SetText (Variables|/Game/Characters/Player/DebugWidget/WBP_DebugSpeed.WBP_DebugSpeed_C|GetLocalSpeed _aswbp_debug_speed) (Utilities|Text|ToText(Float) (Variables|/Script/Engine.CharacterMovementComponent|GetMaxWalkSpeed (Variables|Character|GetCharacterMovement)) "HalfToEven")))

(event EventBeginPlay
  (if (Pawn|IsLocallyControlled)
    (Utilities|FlowControl|Delay 0.2)
    (Networking|SwitchHasAuthority
      (:Authority
        (Class|BNMonoCharacter|BroadcastInitialValues))
      (:Remote
        (CallFunction|ClientInitDelay)))))

(fn ConstructionScript)