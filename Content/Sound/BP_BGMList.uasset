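; BP_BGMList is a background music player that plays tracks from a sound list through its Audio component.
; On BeginPlay it starts the track at the current index and binds to the component's audio-finished event.
; Each time a track finishes, it picks a random index from the whole list and plays that sound, so playback continues and the same track can repeat.
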(event Custom|IndexSetting
  (bind _audio (Variables|Default|GetAudio))
  (Variables|Default|SetCurrentIndex (Math|Random|RandomIntegerinRange 0 (- (Utilities|Array|Length (Variables|Default|GetAudioList)) 1)))
  (Audio|Components|Audio|SetSound _audio (Utilities|Array|Get(acopy) (Variables|Default|GetAudioList) (Variables|Default|GetCurrentIndex)))
  (Audio|Components|Audio|Play _audio 0.0))

(event EventBeginPlay
  (bind _audio (Variables|Default|GetAudio))
  (Audio|Components|Audio|SetSound _audio (Utilities|Array|Get(acopy) (Variables|Default|GetAudioList) (Variables|Default|GetCurrentIndex)))
  (Audio|Components|Audio|Play _audio 0.0)
  (EventDispatchers|BindEventtoOnAudioFinished _audio (delegate Custom|IndexSetting)))

(fn ConstructionScript)