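; BP_MissionPortal is a portal actor that gathers players in its capsule and sends them into a mission of its TransferTo type.
; On the server, overlaps edit the replicated player list and open or close mission widgets, which refresh via OnRep.
; When ready players match the type's quota, matching PlayerStates go to the GameMode's LoadMissionLevel and the started flag and material toggle.
; Assignable missions skip the ready check and already-started guard.
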(event OnComponentBeginOverlap(Capsule)
  (params (OverlappedComponent :type Primitive%20Component%20Object%20Reference) (OtherActor :type Actor%20Object%20Reference) (OtherComp :type Primitive%20Component%20Object%20Reference) (OtherBodyIndex :type Integer) (bFromSweep :type Boolean) (SweepResult :type Hit%20Result%20Structure%20%28by%20ref%29))
  (Networking|SwitchHasAuthority
    (:Authority
      (bind _asbp_test_mono (Utilities|Casting|CastToBP_TestMonoBackView OtherActor))
      (bind _asbp_player_controller (Utilities|Casting|CastToBP_PlayerController (Pawn|GetController _asbp_test_mono)))
      (Utilities|Array|Add (Variables|Default|GetMissionPlayerList) (Utilities|Struct|MakeST_MissionPlayer (PlayerState|GetPlayerName (Variables|/Script/Engine.Controller|GetPlayerState _asbp_player_controller)) false))
      (Default|CreateMissionWidget _asbp_player_controller (Variables|Default|GetTransferTo) (Variables|Default|GetMissionPlayerList))
      (CallFunction|ServerUpdateMissionPlayerList))))

(event OnComponentEndOverlap(Capsule)
  (params (OverlappedComponent :type Primitive%20Component%20Object%20Reference) (OtherActor :type Actor%20Object%20Reference) (OtherComp :type Primitive%20Component%20Object%20Reference) (OtherBodyIndex :type Integer))
  (Networking|SwitchHasAuthority
    (:Authority
      (bind _asbp_test_mono (Utilities|Casting|CastToBP_TestMonoBackView OtherActor))
      (bind _asbp_player_controller (Utilities|Casting|CastToBP_PlayerController (Pawn|GetController _asbp_test_mono)))
      (Utilities|Array|RemoveItem (Variables|Default|GetMissionPlayerList) (Utilities|Struct|MakeST_MissionPlayer (PlayerState|GetPlayerName (Variables|/Script/Engine.Controller|GetPlayerState _asbp_player_controller)) false))
      (Utilities|Array|RemoveItem (Variables|Default|GetMissionPlayerList) (Utilities|Struct|MakeST_MissionPlayer (PlayerState|GetPlayerName (Variables|/Script/Engine.Controller|GetPlayerState _asbp_player_controller)) true))
      (Default|CloseMissionWidget _asbp_player_controller)
      (CallFunction|ServerUpdateMissionPlayerList))))

(event Custom|SetMissionPlayerList
  (params (NewPlayerList :type Array%20of%20ST%20Mission%20Player%20Structures))
  (bind _output_get (Variables|Default|SetMissionPlayerList NewPlayerList))
  (for (_array_element _array_index) _output_get
    (if (.breadystate _array_element)
      (Math|Integer|IncrementInt (Variables|Default|GetReadyCount)
        (:%20%20
          (Utilities|Array|Add (Variables|Default|GetReadyPlayerIndex) _array_index)))))
  (CallFunction|CheckReadyComplete))

(event Custom|Server_UpdateMissionPlayerList
  (CallFunction|UpdateMissionPlayerList))

(event Custom|MoveToMissionArea
  (switch Utilities|FlowControl|Switch|SwitchonE_MissionType (Variables|Default|GetTransferTo)
    (:NewEnumerator0
      (if (not (Variables|Default|GetIsAlreadyStart)) :!label _label
        (bind _asbp_in_game_game_mode (Utilities|Casting|CastToBP_InGameGameMode (Game|GetGameMode) :!label _label_2))
        (Default|LoadMissionLevel _asbp_in_game_game_mode (Variables|Default|GetTransferTo) (Variables|Default|GetMissionPlayerState))
        (CallFunction|SetIsAlreadyStart)))
    (:NewEnumerator1
      (goto _label))
    (:NewEnumerator2
      (goto _label))
    (:NewEnumerator3
      (goto _label_2))))

(event Custom|CheckReadyComplete
  (switch Utilities|FlowControl|Switch|SwitchonE_MissionType (Variables|Default|GetTransferTo)
    (:NewEnumerator0
      (if (== (Variables|Default|GetReadyCount) (Variables|Default|GetMaxReadtCount)) :!label _label
        (bind _outactors (Actor|GetAllActorsOfClass "/Game/GameFramework/PlayerState/BP_PlayerState.BP_PlayerState_C"))
        (for _array_element _outactors
          (for _array_element_2 (Variables|Default|GetReadyPlayerIndex)
            (if (Utilities|Enum|Equal(Enum) (.playername (Utilities|Array|Get(acopy) (Variables|Default|GetMissionPlayerList) _array_element_2)) (PlayerState|GetPlayerName _array_element))
              (Utilities|Array|Add (Variables|Default|GetMissionPlayerState) _array_element))))
        (Variables|Default|SetReadyCount 0)
        (Utilities|Array|Clear (Variables|Default|GetReadyPlayerIndex))
        (CallFunction|MovetoMissionArea)
        (else
          (Variables|Default|SetReadyCount 0)
          (Utilities|Array|Clear (Variables|Default|GetReadyPlayerIndex)))))
    (:NewEnumerator1
      (goto _label))
    (:NewEnumerator2
      (goto _label))
    (:NewEnumerator3
      (CallFunction|MovetoMissionArea))))

(event Custom|SetIsAlreadyStart
  (if (Variables|Default|GetIsAlreadyStart)
    (Variables|Default|SetIsAlreadyStart false)
    (Rendering|Material|SetMaterial (Variables|Default|GetStaticMesh) 0 "/Engine/EditorMaterials/WorldGridPreviewMaterial.WorldGridPreviewMaterial")
    (else
      (Variables|Default|SetIsAlreadyStart true)
      (Rendering|Material|SetMaterial (Variables|Default|GetStaticMesh) 0 "/Engine/VREditor/BasicMeshes/MI_Cube_03.MI_Cube_03"))))

(event EventBeginPlay
  (switch Utilities|FlowControl|Switch|SwitchonE_MissionType (Variables|Default|GetTransferTo)
    (:NewEnumerator0
      (Variables|Default|SetMaxReadtCount 1))
    (:NewEnumerator1
      (Variables|Default|SetMaxReadtCount 2 :!label _label))
    (:NewEnumerator2
      (goto _label))
    (:NewEnumerator3
      (Variables|Default|SetMaxReadtCount 999))))

(fn ConstructionScript)

(fn UpdateMissionPlayerList
  (bind _outactors (Actor|GetAllActorsOfClass "/Game/GameFramework/PlayerController/BP_PlayerController.BP_PlayerController_C"))
  (for _array_element _outactors
    (if (Pawn|IsLocalPlayerController _array_element)
      (Utilities|IsValid (Variables|/Game/GameFramework/PlayerController/BP_PlayerController.BP_PlayerController_C|GetMissionWidget _array_element)
        (:Is%20Valid
          (Default|SetPlayerList (Variables|/Game/GameFramework/PlayerController/BP_PlayerController.BP_PlayerController_C|GetMissionWidget _array_element) (Variables|Default|GetMissionPlayerList)))))))

(fn OnRepMissionPlayerList
  (CallFunction|UpdateMissionPlayerList))