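; BP_AssignableMission_EscapeGate_Test is a test escape gate mission actor that lets prey escape.
; It starts off at BeginPlay, and its On and Off events toggle the Box overlap collision and Niagara effect together through SetVisibilityAndCollision.
; While on, a BP_TestMono overlapping the Box triggers PreyEscape on BP_InGameGameMode.
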(event OnComponentBeginOverlap(Box)
  (params (OverlappedComponent :type Primitive%20Component%20Object%20Reference) (OtherActor :type Actor%20Object%20Reference) (OtherComp :type Primitive%20Component%20Object%20Reference) (OtherBodyIndex :type Integer) (bFromSweep :type Boolean) (SweepResult :type Hit%20Result%20Structure%20%28by%20ref%29))
  (Utilities|Casting|CastToBP_TestMono OtherActor)
  (bind _asbp_in_game_game_mode (Utilities|Casting|CastToBP_InGameGameMode (Game|GetGameMode)))
  (Default|PreyEscape _asbp_in_game_game_mode))

(event Custom|Off
  (CallFunction|SetVisibilityandCollision false))

(event Custom|On
  (CallFunction|SetVisibilityandCollision true))

(event Custom|SetVisibilityAndCollision
  (params (IsOn :type Boolean))
  (bind _niagara (Variables|Default|GetNiagara))
  (bind _niagara_2 (Variables|Default|GetNiagara))
  (if IsOn
    (Collision|SetCollisionEnabled (Variables|Default|GetBox) "QueryOnly")
    (Components|Activation|SetActive _niagara_2 true false)
    (Rendering|SetVisibility _niagara_2 true false)
    (else
      (Collision|SetCollisionEnabled (Variables|Default|GetBox) "NoCollision")
      (Components|Activation|SetActive _niagara false false)
      (Rendering|SetVisibility _niagara false false))))

(event EventBeginPlay
  (CallFunction|Off))

(fn ConstructionScript)