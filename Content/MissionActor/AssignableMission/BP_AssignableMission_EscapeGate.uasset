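; Escape gate mission actor that lets the prey escape once it is revealed.
; It starts with its mesh hidden, trigger collision off and Niagara effect inactive, until SetVisibilltyAndCollision turns all three on.
; When a BP_TestMono overlaps the query-only EscapeTrigger, it calls PreyEscape on BP_InGameGameMode.
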(event OnComponentBeginOverlap(EscapeTrigger)
  (params (OverlappedComponent :type Primitive%20Component%20Object%20Reference) (OtherActor :type Actor%20Object%20Reference) (OtherComp :type Primitive%20Component%20Object%20Reference) (OtherBodyIndex :type Integer) (bFromSweep :type Boolean) (SweepResult :type Hit%20Result%20Structure%20%28by%20ref%29))
  (Utilities|Casting|CastToBP_TestMono OtherActor)
  (bind _asbp_in_game_game_mode (Utilities|Casting|CastToBP_InGameGameMode (Game|GetGameMode)))
  (Default|PreyEscape _asbp_in_game_game_mode))

(event Custom|SetVisibilltyAndCollision
  (Rendering|SetVisibility (Variables|Default|GetStaticMeshComponent) true false)
  (Collision|SetCollisionEnabled (Variables|Default|GetEscapeTrigger) "QueryOnly")
  (Components|Activation|SetActive (Variables|Default|GetNiagaraComponent) true false))

(event EventBeginPlay
  (Rendering|SetVisibility (Variables|Default|GetStaticMeshComponent) false false)
  (Collision|SetCollisionEnabled (Variables|Default|GetEscapeTrigger) "NoCollision")
  (Components|Activation|SetActive (Variables|Default|GetNiagaraComponent) false false))

(fn ConstructionScript)