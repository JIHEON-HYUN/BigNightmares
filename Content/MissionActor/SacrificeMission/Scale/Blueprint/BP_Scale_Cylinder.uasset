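; BP_Scale_Cylinder is the balance beam of a sacrifice-mission scale, tilting its plane mesh according to left and right weight counters.
; Each tick it picks a rotation state from pitch limits and weight difference, interpolating toward a tilt at speed scaled by imbalance, or back to level when equal.
; Reaching either limit detaches that side's registered BP_Scale_Pan and disables the beam's tick.
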(event EventTick
  (params (DeltaSeconds :type Float%20%28single-precision%29))
  (CallFunction|SetRotationState (Variables|Default|GetMax%20Range))
  (switch Utilities|FlowControl|Switch|SwitchonE_RotationState (Variables|Default|GetRotationState)
    (:NewEnumerator0
      (CallFunction|RotatePlane (* -1.0 (Variables|Default|GetAmount)) (Variables|Default|GetSpeed) "NewEnumerator0"))
    (:NewEnumerator1
      (CallFunction|RotatePlane (Variables|Default|GetAmount) (Variables|Default|GetSpeed) "NewEnumerator1"))
    (:NewEnumerator2
      (bind _asbp_scale_pan (Utilities|Casting|CastToBP_Scale_Pan (Variables|Default|GetChildLeft)))
      (Default|DetachComponent _asbp_scale_pan)
      (Actor|Tick|SetActorTickEnabled false))
    (:NewEnumerator3
      (bind _asbp_scale_pan_2 (Utilities|Casting|CastToBP_Scale_Pan (Variables|Default|GetChildRight)))
      (Default|DetachComponent _asbp_scale_pan_2)
      (Actor|Tick|SetActorTickEnabled false))
    (:NewEnumerator4
      (CallFunction|RotatePlane 0.0 1.0 "NewEnumerator4"))))

(fn ConstructionScript)

(fn GetPlaneComponent
  (return (Variables|Default|GetSM_Scale_Plane)))

(fn SetWeightLeft
  (params (AddWeight :type Boolean))
  (if AddWeight
    (Math|Integer|IncrementInt (Variables|Default|GetWeightLeft))
    (else
      (Math|Integer|DecrementInt (Variables|Default|GetWeightLeft)))))

(fn SetWeightRight
  (params (AddWeight :type Boolean))
  (if AddWeight
    (Math|Integer|IncrementInt (Variables|Default|GetWeightRight))
    (else
      (Math|Integer|DecrementInt (Variables|Default|GetWeightRight)))))

(fn SetChild
  (params (ChildActor :type Actor%20Object%20Reference) (IsLeft :type Boolean))
  (if IsLeft
    (Variables|Default|SetChildLeft ChildActor)
    (else
      (Variables|Default|SetChildRight ChildActor))))

(fn SetRotationState
  (params (MaxRange :type Float%20%28double-precision%29))
  (bind _sm_scale_plane (Variables|Default|GetSM_Scale_Plane))
  (bind _returnvalue (Transformation|GetWorldRotation _sm_scale_plane))
  (LocalVariables|SetMaxRangeValue MaxRange)
  (if (or (<= (.pitch _returnvalue) (* -1.0 (LocalVariables|GetMaxRangeValue))) (>= (.pitch _returnvalue) (LocalVariables|GetMaxRangeValue)))
    (if (<= (.pitch _returnvalue) (* -1.0 (LocalVariables|GetMaxRangeValue)))
      (Variables|Default|SetRotationState "NewEnumerator2")
      (else
        (Variables|Default|SetRotationState "NewEnumerator3")))
    (elif (== (- (Variables|Default|GetWeightLeft) (Variables|Default|GetWeightRight)) 0)
      (Variables|Default|SetRotationState "NewEnumerator4")
      (elif (> (- (Variables|Default|GetWeightLeft) (Variables|Default|GetWeightRight)) 0)
        (Variables|Default|SetRotationState "NewEnumerator0")
        (else
          (Variables|Default|SetRotationState "NewEnumerator1"))))))

(fn RotatePlane
  (params (Amount :type Float%20%28double-precision%29) (Speed :type Float%20%28double-precision%29) (State :type E_RotationState%20Enum :default "NewEnumerator0"))
  (LocalVariables|SetRotationAmount Amount)
  (LocalVariables|SetRotationSpeed Speed)
  (switch Utilities|FlowControl|Switch|SwitchonE_RotationState State
    (:NewEnumerator0
      (Transformation|SetWorldRotation (Variables|Default|GetSM_Scale_Plane) (Math|Interpolation|RInterpTo (Transformation|GetWorldRotation (Variables|Default|GetSM_Scale_Plane)) (Math|Rotator|MakeRotator 0.0 (LocalVariables|GetRotationAmount) 9e+01) (Utilities|Time|GetWorldDeltaSeconds) (* (LocalVariables|GetRotationSpeed) (Math|Float|Absolute(Float) (Math|Conversions|ToFloat(Integer) (- (Variables|Default|GetWeightLeft) (Variables|Default|GetWeightRight)))))) false false :!label _label))
    (:NewEnumerator1
      (goto _label))
    (:NewEnumerator4
      (Transformation|SetWorldRotation (Variables|Default|GetSM_Scale_Plane) (Math|Interpolation|RInterpTo (Transformation|GetWorldRotation (Variables|Default|GetSM_Scale_Plane)) "0.000000,90.000000,0.000000" (Utilities|Time|GetWorldDeltaSeconds) (LocalVariables|GetRotationSpeed)) false false))))