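; One pan of the balance scale in the sacrifice mission, attached on BeginPlay to a socket on its parent BP_Scale_Cylinder and registered as left or right.
; Tick zeroes its world rotation so the pan stays level.
; Any overlap starting or ending on its collision component sets or clears that side's weight flag on the cylinder, without filtering or counting.
; DetachComponent releases the pan and enables physics on its circle mesh.
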(event OnComponentBeginOverlap(SM_Scale_Collision)
  (params (OverlappedComponent :type Primitive%20Component%20Object%20Reference) (OtherActor :type Actor%20Object%20Reference) (OtherComp :type Primitive%20Component%20Object%20Reference) (OtherBodyIndex :type Integer) (bFromSweep :type Boolean) (SweepResult :type Hit%20Result%20Structure%20%28by%20ref%29))
  (if (Variables|Default|GetIsLeft)
    (bind _asbp_scale_cylinder (Utilities|Casting|CastToBP_Scale_Cylinder (Variables|Default|GetParentActor)))
    (Default|SetWeightLeft _asbp_scale_cylinder true)
    (else
      (bind _asbp_scale_cylinder_2 (Utilities|Casting|CastToBP_Scale_Cylinder (Variables|Default|GetParentActor)))
      (Default|SetWeightRight _asbp_scale_cylinder_2 true))))

(event OnComponentEndOverlap(SM_Scale_Collision)
  (params (OverlappedComponent :type Primitive%20Component%20Object%20Reference) (OtherActor :type Actor%20Object%20Reference) (OtherComp :type Primitive%20Component%20Object%20Reference) (OtherBodyIndex :type Integer))
  (if (Variables|Default|GetIsLeft)
    (bind _asbp_scale_cylinder (Utilities|Casting|CastToBP_Scale_Cylinder (Variables|Default|GetParentActor)))
    (Default|SetWeightLeft _asbp_scale_cylinder false)
    (else
      (bind _asbp_scale_cylinder_2 (Utilities|Casting|CastToBP_Scale_Cylinder (Variables|Default|GetParentActor)))
      (Default|SetWeightRight _asbp_scale_cylinder_2 false))))

(event Custom|DetachComponent
  (Transformation|DetachFromComponent (Variables|Default|GetDefaultSceneRoot) "KeepRelative" "KeepRelative" "KeepRelative" true)
  (Physics|SetSimulatePhysics (Variables|Default|GetSM_Scale_Circle) true))

(event EventBeginPlay
  (bind _asbp_scale_cylinder (Utilities|Casting|CastToBP_Scale_Cylinder (Variables|Default|GetParentActor)))
  (bind _newparam (Default|GetPlaneComponent _asbp_scale_cylinder))
  (Transformation|AttachComponentToComponent _newparam (Variables|Default|GetSocket%20Name) "SnapToTarget" "KeepWorld" "KeepRelative" true)
  (Default|SetChild _asbp_scale_cylinder self (Variables|Default|GetIsLeft)))

(event EventTick
  (params (DeltaSeconds :type Float%20%28single-precision%29))
  (Transformation|SetActorRotation "0, 0, 0"))

(fn ConstructionScript)