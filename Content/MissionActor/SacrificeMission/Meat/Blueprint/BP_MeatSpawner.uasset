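; BP_MeatSpawner is a Sacrifice mission actor that keeps spawning BP_Meat actors around its Sphere component for as long as it runs.
; From BeginPlay, StartSpawnMeat waits a random interval between the configured minimum and maximum, then OnSpawnMeat spawns one and restarts the cycle.
; Random X and Y offsets within SpawnRadius form a square area at the Sphere's height, and each meat copies the Sphere's rotation and scale.
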(event Custom|StartSpawnMeat
  (Utilities|FlowControl|Delay (Math|Random|RandomFloatinRange (Variables|Default|GetMinSpawnInterval) (Variables|Default|GetMaxSpawnInterval)))
  (CallFunction|OnSpawnMeat))

(event Custom|OnSpawnMeat
  (bind _sphere (Variables|Default|GetSphere))
  (bind _spawnradius (Variables|Default|GetSpawnRadius))
  (bind _spawnradius_2 (Variables|Default|GetSpawnRadius))
  (bind _returnvalue (Transformation|GetWorldTransform _sphere))
  (bind _returnvalue_2 (* -1.0 _spawnradius))
  (bind _returnvalue_3 (Math|Random|RandomFloatinRange _returnvalue_2 _spawnradius_2))
  (Game|SpawnActorfromClass "/Game/MissionActor/SacrificeMission/Meat/Blueprint/BP_Meat.BP_Meat_C" (Math|Transform|MakeTransform (Math|Vector|MakeVector (+ _returnvalue_3 (.x (.location _returnvalue))) (+ _returnvalue_3 (.y (.location _returnvalue))) (.z (.location _returnvalue))) (.rotation _returnvalue) (.scale _returnvalue)) "Undefined" "MultiplyWithRoot" 0 0)
  (CallFunction|StartSpawnMeat))

(event EventBeginPlay
  (CallFunction|StartSpawnMeat))

(fn ConstructionScript)